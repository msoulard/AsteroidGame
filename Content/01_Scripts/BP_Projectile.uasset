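; BP_Projectile is a projectile that flies straight ahead and destroys asteroids it touches.
; Tick moves it along its forward vector by Speed each frame, without sweeping or delta-time scaling.
; An overlap on Sphere1 with a BP_Asteroid destroys both actors, and other overlapping actors are ignored.
; A timer set on BeginPlay destroys the projectile after ten seconds if it is still alive.
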(event `self.ReceiveBeginPlay`
  (`KismetSystemLibrary.K2_SetTimerDelegate` (delegate `E_Death`) 10.0))

(event `E_Death`
  (`self.K2_DestroyActor`))

(event `self.ReceiveTick`
  (params (DeltaSeconds :type "Float (single-precision)"))
  (`self.K2_SetActorLocation` (+ (`self.K2_GetActorLocation`) (* (`self.ForwardVector`) (`self.Speed`)))))

(event `self.Sphere1.OnComponentBeginOverlap`
  (params (OverlappedComponent :type "PrimitiveComponent Object Reference") (OtherActor :type "Actor Object Reference") (OtherComp :type "PrimitiveComponent Object Reference") (OtherBodyIndex :type Integer) (bFromSweep :type Boolean) (SweepResult :type "HitResult Structure (by ref)"))
  (bind _asbp_asteroid (cast `/Game/01_Scripts/BP_Asteroid` OtherActor))
  (`self.K2_DestroyActor` _asbp_asteroid)
  (`self.K2_DestroyActor`))

(fn `UserConstructionScript`)