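; BP_Asteroid is an asteroid actor that drifts in a random horizontal direction and can be destroyed by a hit.
; BeginPlay builds the direction from random unit vector components with zero Z and starts a ten-second self-destruct timer.
; Tick offsets the location by direction times Speed, without delta-time scaling or sweep.
; E_Hit fires the EDDestroyed dispatcher before destroying the actor, while timer expiry destroys it silently.
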(event `self.ReceiveBeginPlay`
  (bind (_returnvalue_x _returnvalue_y) (`KismetMathLibrary.BreakVector` (`KismetMathLibrary.RandomUnitVector`)))
  (set `self.ForwardVector` (`KismetMathLibrary.MakeVector` _returnvalue_x _returnvalue_y))
  (`KismetSystemLibrary.K2_SetTimerDelegate` (delegate `E_Death`) 10.0))

(event `E_Death`
  (`self.K2_DestroyActor`))

(event `self.ReceiveTick`
  (params (DeltaSeconds :type "Float (single-precision)"))
  (`self.K2_SetActorLocation` (+ (`self.K2_GetActorLocation`) (* (`self.ForwardVector`) (`self.Speed`)))))

(event `E_Hit`
  (`self.ED_Destroyed` self)
  (`self.K2_DestroyActor`))

(fn `UserConstructionScript`)