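; BP_ScoreManager tracks the player's score for destroyed asteroids.
; On BeginPlay it registers itself on the game instance and retries on a short delay until the AsteroidManager is valid, then binds to its asteroid-destroyed dispatcher.
; Each destruction adds points by asteroid type, with smaller asteroids worth more, and pushes the new total to the main UI through the game instance.
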(event `self.ReceiveBeginPlay`
  (bind _gameinstance (`/Game/01_Scripts/BP_Utils.F_GetGameinstance`))
  (bind _asteroidmanager (`/Game/01_Scripts/BP_GameInstance.AsteroidManager` _gameinstance))
  (set `/Game/01_Scripts/BP_GameInstance.ScoreManager` self _gameinstance)
  (`/Engine/EditorBlueprintResources/StandardMacros.IsValid` _asteroidmanager :!label _label
    (:`Is Valid`
      (add `/Game/01_Scripts/BP_AsteroidManager.ED_AsteroidDestroyed` _asteroidmanager (delegate `E_ActionOnAsteroidDestroyed`)))
    (:`Is Not Valid`
      (`KismetSystemLibrary.Delay` 0.2)
      (goto _label))))

(event `E_ActionOnAsteroidDestroyed`
  (params (AsteroidType :type "/Game/01_Scripts/Enums/E_AsteroidType Enum" :default "NewEnumerator0"))
  (`self.F_AddScore` AsteroidType)
  (`/Game/04_Widgets/UI_Main.F_SetScore` (`/Game/01_Scripts/BP_GameInstance.UIMain` (`/Game/01_Scripts/BP_Utils.F_GetGameinstance`)) (`self.Score`)))

(event `self.ReceiveTick`
  (params (DeltaSeconds :type "Float (single-precision)")))

(fn `F_AddScore`
  (params (AsteroidType :type "/Game/01_Scripts/Enums/E_AsteroidType Enum" :default "NewEnumerator0"))
  (switch `/Game/01_Scripts/Enums/E_AsteroidType` AsteroidType
    (:`NewEnumerator0`
      (set `self.Score` (+ (`self.Score`) 25)))
    (:`NewEnumerator1`
      (set `self.Score` (+ (`self.Score`) 50)))
    (:`NewEnumerator2`
      (set `self.Score` (+ (`self.Score`) 100)))))

(fn `UserConstructionScript`)