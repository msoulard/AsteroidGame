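; Player pawn for an asteroid game, managing lives and forwarding thrust, rotation and fire inputs to movement and fire components while active.
; BeginPlay polls the game instance for the main UI, then caches the spawn transform and binds full reset to the replay dispatcher.
; Asteroid overlaps, or debug key K, remove a life, then either trigger game over or briefly hide the pawn and respawn it at its start location.
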(event OnComponentBeginOverlap(Box)
  (params (OverlappedComponent :type Primitive%20Component%20Object%20Reference) (OtherActor :type Actor%20Object%20Reference) (OtherComp :type Primitive%20Component%20Object%20Reference) (OtherBodyIndex :type Integer) (bFromSweep :type Boolean) (SweepResult :type Hit%20Result%20Structure%20%28by%20ref%29))
  (bind _root (Variables|Default|GetRoot))
  (Utilities|Casting|CastToBP_Asteroid OtherActor)
  (if (Variables|Default|GetIsActive)
    (bind _result (Math|Integer|DecrementInt (Variables|Default|GetVie))
      (:%20%20
        (Default|FSetVie (Variables|Default|GetUIMain) (Math|Integer|Clamp(Integer) _result 0 3))
        (if (== (Variables|Default|GetVie) 0)
          (Variables|Default|SetIsActive false)
          (Default|FSetGameOver (Variables|Default|GetUIMain) "Visible")
          (Default|FSetVie (Variables|Default|GetUIMain))
          (Default|EGameOver (CallFunction|FGetGameinstance))
          (else
            (Variables|Default|SetIsActive false)
            (Rendering|SetVisibility _root false true)
            (Utilities|FlowControl|Delay 1.0)
            (Transformation|SetActorLocation (Variables|Default|GetDefaultLocation) false false)
            (Rendering|SetVisibility _root true true)
            (Variables|Default|SetIsActive true)))))))

(event Custom|E_Rotate
  (params (InputValue :type Float%20%28double-precision%29))
  (if (Variables|Default|GetIsActive)
    (Default|FRotate (Variables|Default|GetBPC_Movement) InputValue)))

(event Custom|E_SetTargetForwardValue
  (params (InputValue :type Float%20%28double-precision%29))
  (bind _bpc_movement (Variables|Default|GetBPC_Movement))
  (if (Variables|Default|GetIsActive)
    (Default|FSetTargetForwardValue _bpc_movement InputValue)
    (Default|FSetTargetForwardVector _bpc_movement)))

(event Custom|E_ResetPawn
  (CallFunction|FResetPawn))

(event Custom|E_Fire
  (if (Variables|Default|GetIsActive)
    (Default|FFire (Variables|Default|GetBPC_Fire))))

(event EventBeginPlay
  (Utilities|IsValid (Variables|/Game/01_Scripts/BP_GameInstance.BP_GameInstance_C|GetUIMain (CallFunction|FGetGameinstance)) :!label _label
    (:Is%20Valid
      (Variables|Default|SetUIMain (Variables|/Game/01_Scripts/BP_GameInstance.BP_GameInstance_C|GetUIMain (CallFunction|FGetGameinstance)))
      (Default|FSetVie (Variables|/Game/01_Scripts/BP_GameInstance.BP_GameInstance_C|GetUIMain (CallFunction|FGetGameinstance)) (Variables|Default|GetVie))
      (Variables|Default|SetDefaultLocation (Transformation|GetActorLocation))
      (Variables|Default|SetDefaultRotation (Transformation|GetActorRotation))
      (EventDispatchers|BindEventtoEDReplay (CallFunction|FGetGameinstance) (delegate Custom|E_ResetPawn)))
    (:Is%20Not%20Valid
      (Utilities|FlowControl|Delay 0.2)
      (goto _label))))

(event Input|KeyboardEvents|DebugKeyK
  (params (Key :type Key%20Structure :default "None") (ActionValue :type Input%20Action%20Value%20Structure))
  (bind _root (Variables|Default|GetRoot))
  (:Pressed
    (if (Variables|Default|GetIsActive)
      (bind _result (Math|Integer|DecrementInt (Variables|Default|GetVie))
        (:%20%20
          (Default|FSetVie (Variables|Default|GetUIMain) (Math|Integer|Clamp(Integer) _result 0 3))
          (if (== (Variables|Default|GetVie) 0)
            (Variables|Default|SetIsActive false)
            (Default|FSetGameOver (Variables|Default|GetUIMain) "Visible")
            (Default|FSetVie (Variables|Default|GetUIMain))
            (Default|EGameOver (CallFunction|FGetGameinstance))
            (else
              (Variables|Default|SetIsActive false)
              (Rendering|SetVisibility _root false true)
              (Utilities|FlowControl|Delay 1.0)
              (Transformation|SetActorLocation (Variables|Default|GetDefaultLocation) false false)
              (Rendering|SetVisibility _root true true)
              (Variables|Default|SetIsActive true))))))))

(fn ConstructionScript)

(fn FResetPawn
  (Transformation|SetActorLocation (Variables|Default|GetDefaultLocation) false false)
  (Transformation|SetActorRotation (Variables|Default|GetDefaultRotation))
  (Variables|Default|SetVie 3)
  (Default|FSetVie (Variables|Default|GetUIMain) (Variables|Default|GetVie))
  (Variables|Default|SetIsActive true))