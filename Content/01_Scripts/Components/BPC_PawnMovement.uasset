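; Pawn movement component that gives its owner throttle-style motion with inertia and drift.
; Input functions adjust a clamped forward target and yaw the pawn, while Tick interpolates toward that target and offsets the location without sweep.
; A separate function eases the travel vector toward the actor's facing at a quarter of the throttle's interpolation speed.
; An unfinished screen-edge wrap, mixing viewport pixels with world coordinates, is disconnected from execution.
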(event `self.ReceiveBeginPlay`
  (`parent.ReceiveBeginPlay`)
  (set `self.DefaultLocation` (`Actor.K2_GetActorLocation` (`self.PawnOwner`))))

(event `self.ReceiveTick`
  (params (DeltaSeconds :type "Float (single-precision)"))
  (`self.F_Move`))

(fn `F_Move`
  (bind _output_get (set `self.CurrentForwardValue` (`KismetMathLibrary.FInterpTo` (`self.CurrentForwardValue`) (`self.TargetForwardValue`) (`GameplayStatics.GetWorldDeltaSeconds`) (`self.ForwardInterpolationSpeed`))))
  (`Actor.K2_SetActorLocation` (`self.PawnOwner`) (+ (`Actor.K2_GetActorLocation` (`self.PawnOwner`)) (* _output_get (`self.CurrentForwardVector`) (`self.Speed`))) false false))

(fn `F_ResetPosition`
  (locals (ValueX_Pawn :type "Float (double-precision)") (ValueY_pawn :type "Float (double-precision)") (OutOfBound :type Boolean))
  (bind (_returnvalue_x _returnvalue_y) (`KismetMathLibrary.BreakVector2D` (`WidgetLayoutLibrary.GetViewportSize`)))
  (bind _returnvalue_x_2 (`KismetMathLibrary.BreakVector2D` (`WidgetLayoutLibrary.GetViewportSize`)))
  (bind (_defaultlocation_x _defaultlocation_y _defaultlocation_z) (`KismetMathLibrary.BreakVector` (`self.DefaultLocation`)))
  (bind _valuex_pawn (`local.ValueX_Pawn`))
  (bind _valuey_pawn (`local.ValueY_pawn`))
  (bind (_defaultlocation_x_2 _defaultlocation_y_2 _defaultlocation_z_2) (`KismetMathLibrary.BreakVector` (`self.DefaultLocation`)))
  (bind _screenlocation (`PlayerController.ProjectWorldLocationToScreen` (`GameplayStatics.GetPlayerController` 0) (`Actor.K2_GetActorLocation` (`self.PawnOwner`)) false))
  (`|ExecutionSequence`
    (:`then_0`
      ;[1 1 1] Get x and y pawn position
      (set `local.ValueX_Pawn` (`KismetMathLibrary.BreakVector2D` _screenlocation))
      (set `local.ValueY_pawn` (`.Y` (`KismetMathLibrary.BreakVector2D` _screenlocation))))
    (:`then_1`
      (if (>= _valuex_pawn _returnvalue_x_2)
        (set `local.ValueX_Pawn` (/ _returnvalue_x_2 -2.0))
        (set `local.OutOfBound` true)
        (elif (< _valuex_pawn 0.0)
          (set `local.ValueX_Pawn` (/ _returnvalue_x_2 2.0))
          (set `local.OutOfBound` true))))
    (:`then_2`
      (if (>= _valuey_pawn _returnvalue_y)
        (set `local.ValueY_pawn` (/ _returnvalue_y -2.0))
        (set `local.OutOfBound` true)
        (elif (< _valuey_pawn 0.0)
          (set `local.ValueY_pawn` (/ _returnvalue_y 2.0))
          (set `local.OutOfBound` true))))
    (:`then_3`
      (if (`local.OutOfBound`)
        (`KismetSystemLibrary.LineTraceSingle` :`Start` (`self.DefaultLocation`) :`End` (`KismetMathLibrary.MakeVector` (`local.ValueX_Pawn`) (`local.ValueY_pawn`) _defaultlocation_z_2) :`TraceChannel` "TraceTypeQuery1" :`DrawDebugType` "Persistent")
        (`Actor.K2_SetActorLocation` (`self.PawnOwner`) (`KismetMathLibrary.MakeVector` (`local.ValueX_Pawn`) (`local.ValueY_pawn`) _defaultlocation_z) false false)))))

(fn `F_Rotate`
  (params (RotateInput :type "Float (double-precision)"))
  (`Actor.K2_SetActorRotation` (`self.PawnOwner`) (`KismetMathLibrary.ComposeRotators` (`Actor.K2_GetActorRotation` (`self.PawnOwner`)) (`KismetMathLibrary.MakeRotator` 0.0 0.0 (* RotateInput (`self.RotationRate`)))) true))

(fn `F_SetTargetForwardValue`
  (params (ForwardInput :type "Float (double-precision)"))
  (locals (DirectionSpeed :type "Float (double-precision)" :default 1.0))
  (set `self.TargetForwardValue` (`KismetMathLibrary.FClamp` (+ (`self.TargetForwardValue`) (* ForwardInput (`local.DirectionSpeed`) (`GameplayStatics.GetWorldDeltaSeconds`))) -1.0)))

(fn `F_SetTargetForwardVector`
  (locals (DirectionSpeed :type "Float (double-precision)" :default 1.0))
  (set `self.CurrentForwardVector` (`KismetMathLibrary.VInterpTo` (`self.CurrentForwardVector`) (`Actor.GetActorForwardVector` (`self.PawnOwner`)) (`GameplayStatics.GetWorldDeltaSeconds`) (/ (`self.ForwardInterpolationSpeed`) 4.0))))