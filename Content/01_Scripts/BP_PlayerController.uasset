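; Player controller that sets up Enhanced Input and relays movement, rotation and fire input to the controlled pawn.
; On BeginPlay it sets Game and UI input with permanent mouse capture, caches the pawn, adds IMC_Player and triggers the game instance's main init if the input subsystem is valid.
; Movement and rotation forward both Triggered and Completed values to the pawn, while fire calls the pawn's fire event.
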(event `self.ReceiveBeginPlay`
  (bind _returnvalue (subsystem `EnhancedInputLocalPlayerSubsystem`))
  (`WidgetBlueprintLibrary.SetInputMode_GameAndUIEx` (`GameplayStatics.GetPlayerController` 0) null)
  (`GameplayStatics.SetViewportMouseCaptureMode` "CapturePermanently_IncludingInitialMouseDown")
  (set `self.ControlledPawn` (`/Game/01_Scripts/BP_Utils.F_GetPawn`))
  (`/Engine/EditorBlueprintResources/StandardMacros.IsValid` _returnvalue
    (:`Is Valid`
      (`EnhancedInputSubsystemInterface.AddMappingContext` _returnvalue "/Game/01_Scripts/Inputs/IMC_Player.IMC_Player" 0 (struct))
      (`/Game/01_Scripts/BP_GameInstance.E_InitMain` (`/Game/01_Scripts/BP_Utils.F_GetGameinstance`)))))

(event `EnhancedInput|/Game/01_Scripts/Inputs/IA_Movement`
  (params (ActionValue :type "Float (double-precision)") (ElapsedSeconds :type "Float (double-precision)") (TriggeredSeconds :type "Float (double-precision)") (InputAction :type "InputAction Object Reference" :default "/Game/01_Scripts/Inputs/IA_Movement.IA_Movement"))
  (bind _controlledpawn (`self.ControlledPawn`))
  (:`Triggered`
    (`/Game/01_Scripts/BP_Pawn.E_SetTargetForwardValue` _controlledpawn ActionValue))
  (:`Completed`
    (`/Game/01_Scripts/BP_Pawn.E_SetTargetForwardValue` _controlledpawn ActionValue)))

(event `EnhancedInput|/Game/01_Scripts/Inputs/IA_Rotation`
  (params (ActionValue :type "Float (double-precision)") (ElapsedSeconds :type "Float (double-precision)") (TriggeredSeconds :type "Float (double-precision)") (InputAction :type "InputAction Object Reference" :default "/Game/01_Scripts/Inputs/IA_Rotation.IA_Rotation"))
  (bind _controlledpawn (`self.ControlledPawn`))
  (:`Triggered`
    (`/Game/01_Scripts/BP_Pawn.E_Rotate` _controlledpawn ActionValue))
  (:`Completed`
    (`/Game/01_Scripts/BP_Pawn.E_Rotate` _controlledpawn ActionValue)))

(event `EnhancedInput|/Game/01_Scripts/Inputs/IA_Fire`
  (params (ActionValue :type Boolean) (ElapsedSeconds :type "Float (double-precision)") (TriggeredSeconds :type "Float (double-precision)") (InputAction :type "InputAction Object Reference" :default "/Game/01_Scripts/Inputs/IA_Fire.IA_Fire"))
  (:`Triggered`
    (`/Game/01_Scripts/BP_Pawn.E_Fire` (`self.ControlledPawn`))))

(fn `UserConstructionScript`)